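; BP_SPIDERMAN is a spider enemy that chases the first player and attacks up close.
; BeginPlay starts an AIMoveTo loop that repeats after each successful move.
; Tick plays the attack montage within range, pausing movement until it completes.
; Any damage lowers clamped Hp, disables movement and collision, and destroys the actor after a delay, though Dead becomes true only at zero Hp.
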(event EventTick
  (params (DeltaSeconds :type Float%20%28single-precision%29))
  (if (CallFunction|IsAlive)
    (if (CallFunction|IsAttackRange)
      (if (not (CallFunction|IsAttacking))
        (Components|Activation|Deactivate (Variables|Character|GetCharacterMovement))
        (Animation|Montage|PlayMontage (Variables|Character|GetMesh) "/Game/Characters/Enemy_Great_Spider/Animations/AM_SpiderAttack.AM_SpiderAttack"
          (:OnCompleted
            (Components|Activation|Activate (Variables|Character|GetCharacterMovement) false)))))))

(event Game|Damage|EventAnyDamage
  (params (Damage :type Float%20%28single-precision%29) (DamageType :type Damage%20Type%20Object%20Reference) (InstigatedBy :type Controller%20Object%20Reference) (DamageCauser :type Actor%20Object%20Reference))
  (bind _output_get (Variables|Default|Sethp (Math|Float|Clamp(Float) (- (Variables|Default|Gethp) Damage) 0.0 1e+02)))
  (CallFunction|KillSpider (== _output_get 0.0))
  (Utilities|FlowControl|Delay 5.0)
  (Actor|DestroyActor))

(event EventBeginPlay
  (if (CallFunction|IsAlive)
    (AI|AIMoveTo self "0, 0, 0" (Game|GetPlayerCharacter 0) 5.0 false :!label _label
      (:OnSuccess
        (Utilities|FlowControl|Delay 0.2)
        (goto _label)))))

(fn ConstructionScript)

(fn IsAttackRange
  (return (< (Transformation|GetDistanceTo (Game|GetPlayerCharacter 0)) (Variables|Default|Getattack%20range))))

(fn IsAttacking
  (return (Animation|Montage|MontageIsPlaying (Components|SkeletalMesh|GetAnimInstance (Variables|Character|GetMesh)) "/Game/Characters/Enemy_Great_Spider/Animations/AM_SpiderAttack.AM_SpiderAttack")))

(fn IsAlive
  (return (not (Variables|Default|Getdead))))

(fn KillSpider
  (params (Dead :type Boolean))
  (Variables|Default|Setdead Dead)
  (Components|Activation|Deactivate (Variables|Character|GetCharacterMovement))
  (Collision|SetActorEnableCollision false))