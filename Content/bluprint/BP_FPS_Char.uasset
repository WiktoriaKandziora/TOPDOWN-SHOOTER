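; Player marine character that creates its HUD, moves on input axes, fires an assault rifle and tracks health until death.
; Mouse velocity beyond a deadzone sets a target yaw from its direction, and control rotation interpolates toward it each tick.
; Holding fire starts muzzle effect and sound and loops a timed line trace from the rifle along control rotation, applying damage.
; Incoming damage reduces clamped health; death stops fire effects and blocks movement, rotation and new firing.
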(event EventTick
  (params (DeltaSeconds :type Float%20%28single-precision%29))
  (if (CallFunction|IsAlive)
    (CallFunction|CharacterRotate)))

(event Game|Damage|EventAnyDamage
  (params (Damage :type Float%20%28single-precision%29) (DamageType :type Damage%20Type%20Object%20Reference) (InstigatedBy :type Controller%20Object%20Reference) (DamageCauser :type Actor%20Object%20Reference))
  (bind _output_get (Variables|Default|Sethealth (Math|Float|Clamp(Float) (- (Variables|Default|Gethealth) Damage) 0.0 1e+02)))
  (bind _output_get_2 (Variables|Default|Setdead (== _output_get 0.0)))
  (if _output_get_2
    (CallFunction|StopFire)))

(event EventBeginPlay
  (bind _returnvalue (UserInterface|CreateWidget "/Game/UMG/W_playerhud.W_playerhud_C" 0 self))
  (UserInterface|Viewport|AddtoViewport _returnvalue 0))

(event Input|ActionEvents|InputActionfire
  (params (Key :type Key%20Structure :default "None"))
  (:Pressed
    (if (CallFunction|IsAlive)
      (CallFunction|StartFire)
      (CallFunction|WeaponTrace)
      (Utilities|Time|SetTimerbyFunctionName 0 "Weapon Trace" 0.08 true)))
  (:Released
    (CallFunction|StopFire)
    (if (CallFunction|IsAlive)
      (Audio|SpawnSound2D "/Game/Sounds/Weapon_AssaultRifle/Stereo/SC_endfire.SC_endfire" 1.0 1.0 0.0 0)
      (Utilities|Time|ClearTimerbyFunctionName 0 "Weapon Trace"))))

(event Input|AxisEvents|InputAxisMoveForwardBack
  (params (AxisValue :type Float%20%28single-precision%29))
  (if (CallFunction|IsAlive)
    (Pawn|Input|AddMovementInput (Math|Vector|GetForwardVector (Variables|Collision|GetCapsuleComponent)) AxisValue false)))

(event Input|AxisEvents|InputAxisMoveLeftRight
  (params (AxisValue :type Float%20%28single-precision%29))
  (if (CallFunction|IsAlive)
    (Pawn|Input|AddMovementInput (Math|Vector|GetRightVector (Variables|Collision|GetCapsuleComponent)) AxisValue false)))

(fn ConstructionScript)

(fn MouseVelocity
  (bind _returnvalue (Game|GetPlayerController 0))
  (bind (_deltax _deltay) (Class|PlayerController|GetInputMouseDelta _returnvalue))
  (return (/ (Math|Vector2D|MakeVector2D _deltax _deltay) (Utilities|Time|GetWorldDeltaSeconds))))

(fn CharacterRotate
  (bind _returnvalue (Game|GetPlayerController 0))
  (bind _returnvalue_2 (CallFunction|MouseVelocity))
  (bind _returnvalue_3 (Class|KismetMathLibrary|DegAtan2 (.x _returnvalue_2) (.y _returnvalue_2)))
  (if (CallFunction|IsMouseDeadZone)
    (Development|PrintString (Utilities|String|ToString(Float) _returnvalue_3) false)
    (Pawn|SetControlRotation _returnvalue (Math|Interpolation|RInterpTo (Pawn|GetControlRotation _returnvalue :!class /Script/Engine.Controller) (Math|Rotator|MakeRotator 0.0 0.0 _returnvalue_3) (Utilities|Time|GetWorldDeltaSeconds) (Variables|Default|Getinterp%20speed)))))

(fn IsMouseDeadZone
  (return (> (Math|Vector2D|Vector2DLength (CallFunction|MouseVelocity)) (Variables|Default|Getdeadzone))))

(fn IsAlive
  (return (not (Variables|Default|Getdead))))

(fn StartFire
  (Components|Activation|Activate (Variables|Default|GetP_AssaultRifle_MF) false)
  (bind _returnvalue (Audio|SpawnSound2D "/Game/Sounds/Weapon_AssaultRifle/Stereo/SC_Weaponfire01.SC_Weaponfire01" 1.0 1.0 0.0 0))
  (Variables|Default|Setwep%20sound _returnvalue))

(fn StopFire
  (bind _wep_sound (Variables|Default|Getwep%20sound))
  (Components|Activation|Deactivate (Variables|Default|GetP_AssaultRifle_MF))
  (Utilities|IsValid _wep_sound
    (:Is%20Valid
      (Audio|Components|Audio|Stop _wep_sound))))

(fn WeaponTrace
  (bind _outhit (Collision|LineTraceByChannel (CallFunction|GetStartLocationLineface) (CallFunction|GetEndLocLINETRACE) "TraceTypeQuery1" false 0 "ForDuration"))
  (Game|Damage|ApplyDamage (.HitActor (Collision|BreakHitResult _outhit)) 15.0 0 0))

(fn GetStartLocationLineface
  (return (Transformation|GetSocketLocation (Variables|Default|Getrifle) "None")))

(fn GetEndLocLINETRACE
  (return (+ (CallFunction|GetStartLocationLineface) (* (Math|Vector|GetForwardVector (Pawn|GetControlRotation :!class /Script/Engine.Pawn)) (Variables|Default|Getweapon%20range)))))